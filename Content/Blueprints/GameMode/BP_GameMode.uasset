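; Game mode Blueprint that handles the start and end screens of a match.
; StartGame puts the start-game widget on screen.
; GameOver shows the end-game widget with win or loss text based on WonGame, then waits briefly before calling ResetCurrentLevel.
; ResetCurrentLevel restarts play by reopening the current level by name, whatever the result.
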(event EventBeginPlay)

(event EventTick
  (params (DeltaSeconds :type Float%20%28single-precision%29)))

(event EventStartGame
  (bind _returnvalue (UserInterface|CreateWidget "/Game/Blueprints/Widgets/WBP_StartGameWidget.WBP_StartGameWidget_C"))
  (UserInterface|Viewport|AddtoViewport _returnvalue 0))

(event EventGameOver
  (params (bWonGame :type Boolean))
  (bind _returnvalue (UserInterface|CreateWidget "/Game/Blueprints/Widgets/WBP_EndGameWidget.WBP_EndGameWidget_C"))
  (UserInterface|Viewport|AddtoViewport _returnvalue 0)
  (if bWonGame
    (Rendering|Components|TextRender|SetText (Variables|/Game/Blueprints/Widgets/WBP_EndGameWidget.WBP_EndGameWidget_C|GetDisplayText _returnvalue) "Congratulations!")
    (Utilities|FlowControl|Delay 3.0)
    (CallFunction|ResetCurrentLevel)
    (else
      (Rendering|Components|TextRender|SetText (Variables|/Game/Blueprints/Widgets/WBP_EndGameWidget.WBP_EndGameWidget_C|GetDisplayText _returnvalue) "You've Lost!")
      (Utilities|FlowControl|Delay 3.0)
      (CallFunction|ResetCurrentLevel))))

(fn ConstructionScript)

(fn ResetCurrentLevel
  (bind _returnvalue (Game|GetCurrentLevelName true))
  (Game|OpenLevel(byName) (Utilities|String|StringToName _returnvalue)))